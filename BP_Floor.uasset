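; Floor actor that positions four camera actors relative to its static mesh bounds when play begins.
; BeginPlay finds the cameras by class and sends each a position built from bounds origin, selected box extents, per-camera X/Y offsets and a shared Z offset.
; The Cam3 offsets feed SetPositionCam4 and the Cam4 offsets feed SetPositionCam3.
; A cast-based SetPosition alternative remains as disconnected, unused logic.
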(event `self.ReceiveBeginPlay`
  (bind (_origin _boxextent) (`KismetSystemLibrary.GetComponentBounds` (`self.StaticMeshComponent`)))
  (bind (_origin_2 _boxextent_2) (`KismetSystemLibrary.GetComponentBounds` (`self.StaticMeshComponent`)))
  (bind (_origin_3 _boxextent_3) (`KismetSystemLibrary.GetComponentBounds` (`self.StaticMeshComponent`)))
  (bind _outactors (`GameplayStatics.GetAllActorsOfClass` null))
  (`self.Set_Position_Cam1` _outactors (+ (.x _origin_3) (`self.Cam1_X_Offset`)) (+ (.y _origin_3) (.y _boxextent_3) (`self.Cam1_Y_Offset`)) (`self.Offset_Z`))
  (bind _outactors_2 (`GameplayStatics.GetAllActorsOfClass` null))
  (`self.Set_Position_Cam2` _outactors_2 (+ (.x _origin_2) (.x _boxextent_2) (`self.Cam2_X_Offset`)) (+ (.y _origin_2) (.y _boxextent_2) (`self.Cam2_Y_Offset`)) (`self.Offset_Z`))
  (bind _outactors_3 (`GameplayStatics.GetAllActorsOfClass` null))
  (`self.Set_Position_Cam4` _outactors_3 (+ (.x (`KismetSystemLibrary.GetComponentBounds` (`self.StaticMeshComponent`))) (`self.Cam3_X_Offset`)) (+ (.y (`KismetSystemLibrary.GetComponentBounds` (`self.StaticMeshComponent`))) (`self.Cam3_Y_Offset`)) (`self.Offset_Z`))
  (bind _outactors_4 (`GameplayStatics.GetAllActorsOfClass` null))
  (`self.Set_Position_Cam3` _outactors_4 (+ (.x _origin) (.x _boxextent) (`self.Cam4_X_Offset`)) (+ (.y _origin) (`self.Cam4_Y_Offset`)) (`self.Offset_Z`)))

(fn `Set_Position`
  (params (Camera :type "Object Object Reference") (Offset_X :type "Float (double-precision)") (Offset_Y :type "Float (double-precision)")))

(fn `UserConstructionScript`)