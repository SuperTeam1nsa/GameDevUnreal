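; Camera4_BP is a camera actor blueprint that can be placed at given coordinates and aimed at a point.
; Its Set_Position_Cam4 event moves the CameraComponent to the X, Y, Z position, rotated to look at the supplied Origin.
; A separate SetHideObject function shows or hides in game every actor tagged HideOnNorthWest, suggesting this camera covers the north-west view.
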(event `Set_Position_Cam4`
  (params (x :type "Float (double-precision)") (y :type "Float (double-precision)") (z :type "Float (double-precision)") (Origin :type "Vector Structure"))
  (bind _returnvalue (`KismetMathLibrary.MakeVector` x y z))
  (`SceneComponent.K2_SetWorldRotation` (`self.CameraComponent`) (`KismetMathLibrary.FindLookAtRotation` _returnvalue Origin) false false)
  (`SceneComponent.K2_SetWorldLocation` (`self.CameraComponent`) _returnvalue false false))

(fn `setHideObject`
  (params (Hide :type Boolean :default false))
  (bind _outactors (`GameplayStatics.GetAllActorsWithTag` "HideOnNorthWest"))
  (for _array_element _outactors
    (`self.SetActorHiddenInGame` _array_element Hide)))

(fn `UserConstructionScript`)