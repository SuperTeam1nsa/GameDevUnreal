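; Floor actor that positions four corner cameras around itself when play begins.
; BeginPlay finds all actors of Camera1_BP through Camera4_BP and calls each type's SetPosition function.
; Each call passes a different corner of the static mesh bounds, pushed outward by X/Y offsets, with Z set to OffsetZ, plus the bounds origin.
; The SetPosition function is empty; its cast-based camera chain is disconnected and has broken casts.
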(event `self.ReceiveBeginPlay`
  (bind (_origin _boxextent) (`KismetSystemLibrary.GetComponentBounds` (`self.StaticMeshComponent`)))
  (bind (_origin_2 _boxextent_2) (`KismetSystemLibrary.GetComponentBounds` (`self.StaticMeshComponent`)))
  (bind (_origin_3 _boxextent_3) (`KismetSystemLibrary.GetComponentBounds` (`self.StaticMeshComponent`)))
  (bind (_origin_4 _boxextent_4) (`KismetSystemLibrary.GetComponentBounds` (`self.StaticMeshComponent`)))
  (bind _outactors (`GameplayStatics.GetAllActorsOfClass` "/Game/Dev/Camera/Camera1_BP.Camera1_BP_C"))
  (`/Game/Dev/Camera/Camera1_BP.Set_Position_Cam1` _outactors (+ (.x _origin_4) (.x _boxextent_4) (`self.Offset_X`)) (- (- (.y _origin_4) (.y _boxextent_4)) (`self.Offset_Y`)) (`self.Offset_Z`) _origin_4)
  (bind _outactors_2 (`GameplayStatics.GetAllActorsOfClass` "/Game/Dev/Camera/Camera2_BP.Camera2_BP_C"))
  (`/Game/Dev/Camera/Camera2_BP.Set_Position_Cam2` _outactors_2 (- (- (.x _origin_2) (.x _boxextent_2)) (`self.Offset_X`)) (- (- (.y _origin_2) (.y _boxextent_2)) (`self.Offset_Y`)) (`self.Offset_Z`) _origin_2)
  (bind _outactors_3 (`GameplayStatics.GetAllActorsOfClass` "/Game/Dev/Camera/Camera3_BP.Camera3_BP_C"))
  (`/Game/Dev/Camera/Camera3_BP.Set_Position_Cam3` _outactors_3 (- (- (.x _origin) (.x _boxextent)) (`self.Offset_X`)) (+ (.y _origin) (.y _boxextent) (`self.Offset_Y`)) (`self.Offset_Z`) _origin)
  (bind _outactors_4 (`GameplayStatics.GetAllActorsOfClass` "/Game/Dev/Camera/Camera4_BP.Camera4_BP_C"))
  (`/Game/Dev/Camera/Camera4_BP.Set_Position_Cam4` _outactors_4 (+ (.x _origin_3) (.x _boxextent_3) (`self.Offset_X`)) (+ (.y _origin_3) (.y _boxextent_3) (`self.Offset_Y`)) (`self.Offset_Z`) _origin_3))

(fn `Set_Position`
  (params (Camera :type "/Game/Dev/Camera/Camera1_BP Object Reference") (Offset_X :type "Float (double-precision)") (Offset_Y :type "Float (double-precision)")))

(fn `UserConstructionScript`)