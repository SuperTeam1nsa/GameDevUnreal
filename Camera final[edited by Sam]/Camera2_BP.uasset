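; Camera2_BP is a camera Blueprint that can be positioned at given coordinates to look at a target point.
; Set_Position_Cam2 moves its CameraComponent to the X, Y, Z location without sweeping and rotates it with a look-at toward Origin.
; SetHideObject shows or hides in game every actor tagged HideOnSouthEast, suggesting these obstruct a south-east view.
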(event `Set_Position_Cam2`
  (params (x :type "Float (double-precision)") (y :type "Float (double-precision)") (z :type "Float (double-precision)") (origin :type "Vector Structure"))
  (bind _returnvalue (`KismetMathLibrary.MakeVector` x y z))
  (`SceneComponent.K2_SetWorldRotation` (`self.CameraComponent`) (`KismetMathLibrary.FindLookAtRotation` _returnvalue origin) false false)
  (`SceneComponent.K2_SetWorldLocation` (`self.CameraComponent`) _returnvalue false false))

(fn `setHideObject`
  (params (hide :type Boolean))
  (bind _outactors (`GameplayStatics.GetAllActorsWithTag` "HideOnSouthEast"))
  (for _array_element _outactors
    (`self.SetActorHiddenInGame` _array_element hide)))

(fn `UserConstructionScript`)