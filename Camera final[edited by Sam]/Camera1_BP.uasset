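; Camera actor Blueprint for a fixed viewpoint, Camera1, whose position is set from outside.
; Set_Position_Cam1 moves the camera component to a given XYZ, aims it at an origin point with a look-at rotation, and prints the position for debugging.
; SetHideObject shows or hides every actor tagged "HideOnSouthWest", suggesting it clears objects for a south-west view.
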(event `Set_Position_Cam1`
  (params (x :type "Float (double-precision)") (y :type "Float (double-precision)") (z :type "Float (double-precision)") (Origin :type "Vector Structure"))
  (bind _returnvalue (`KismetMathLibrary.MakeVector` x y z))
  (`SceneComponent.K2_SetWorldRotation` (`self.CameraComponent`) (`KismetMathLibrary.FindLookAtRotation` _returnvalue Origin) false false)
  (`SceneComponent.K2_SetWorldLocation` (`self.CameraComponent`) _returnvalue false false)
  (`KismetSystemLibrary.PrintString` (`KismetStringLibrary.Conv_VectorToString` _returnvalue)))

(fn `setHideObject`
  (params (Hide :type Boolean))
  (bind _outactors (`GameplayStatics.GetAllActorsWithTag` "HideOnSouthWest"))
  (for _array_element _outactors
    (`self.SetActorHiddenInGame` _array_element Hide)))

(fn `UserConstructionScript`)