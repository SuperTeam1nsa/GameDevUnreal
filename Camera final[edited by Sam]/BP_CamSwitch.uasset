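; BP_CamSwitch cycles the player's view between four fixed camera actors when the SwitchCam input is released, using Left and Right for opposite directions.
; The construction script caches one actor of each camera class through nested GetAllActorsOfClass loops.
; FonctionSwitchCam casts the current view target to pick the next camera, then blends to it and prints a compass label.
; It also enables SetHideObject on the new camera and disables it on both neighbors.
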(event `InputAction|SwitchCam`
  (params (Key :type "Key Structure"))
  (:`Released`
    (`self.fonction_SwitchCam` Key)))

(fn `fonction_SwitchCam`
  (params (Keys :type "Key Structure"))
  (bind _viewtarget (`self.ViewTarget`))
  (bind _output_get (set `self.PlayerController` (`GameplayStatics.GetPlayerController` 0)))
  (set `self.ViewTarget` (`Controller.GetViewTarget` _output_get))
  (if (== Keys "Left")
    (cast `/Game/Dev/Camera/Camera1_BP` _viewtarget
      (:`then`
        (`PlayerController.SetViewTargetWithBlend` (`self.PlayerController`) (`self.Camera4`) 0.0 "VTBlend_Linear" 0.0 false :!label _label)
        (`KismetSystemLibrary.PrintString` "NO")
        (`/Game/Dev/Camera/Camera4_BP.setHideObject` (`self.Camera4`) true)
        (`/Game/Dev/Camera/Camera3_BP.setHideObject` (`self.Camera3`) false)
        (`/Game/Dev/Camera/Camera1_BP.setHideObject` (`self.Camera1`) false))
      (:`CastFailed`
        (cast `/Game/Dev/Camera/Camera2_BP` _viewtarget
          (:`then`
            (`PlayerController.SetViewTargetWithBlend` (`self.PlayerController`) (`self.Camera1`) 0.0 "VTBlend_Linear" 0.0 false :!label _label_2)
            (`KismetSystemLibrary.PrintString` "SO")
            (`/Game/Dev/Camera/Camera1_BP.setHideObject` (`self.Camera1`) true)
            (`/Game/Dev/Camera/Camera4_BP.setHideObject` (`self.Camera4`) false)
            (`/Game/Dev/Camera/Camera2_BP.setHideObject` (`self.Camera2`) false))
          (:`CastFailed`
            (cast `/Game/Dev/Camera/Camera4_BP` _viewtarget
              (:`then`
                (`PlayerController.SetViewTargetWithBlend` (`self.PlayerController`) (`self.Camera3`) 0.0 "VTBlend_Linear" 0.0 false :!label _label_3)
                (`KismetSystemLibrary.PrintString` "NE")
                (`/Game/Dev/Camera/Camera3_BP.setHideObject` (`self.Camera3`) true)
                (`/Game/Dev/Camera/Camera2_BP.setHideObject` (`self.Camera2`) false)
                (`/Game/Dev/Camera/Camera4_BP.setHideObject` (`self.Camera4`) false))
              (:`CastFailed`
                (`PlayerController.SetViewTargetWithBlend` (`self.PlayerController`) (`self.Camera2`) 0.0 "VTBlend_Linear" 0.0 false :!label _label_4)
                (`KismetSystemLibrary.PrintString` "SE")
                (`/Game/Dev/Camera/Camera2_BP.setHideObject` (`self.Camera2`) true)
                (`/Game/Dev/Camera/Camera1_BP.setHideObject` (`self.Camera1`) false)
                (`/Game/Dev/Camera/Camera3_BP.setHideObject` (`self.Camera3`) false)))))))
    (elif (== Keys "Right")
      (cast `/Game/Dev/Camera/Camera1_BP` _viewtarget
        (:`then`
          (goto _label_4))
        (:`CastFailed`
          (cast `/Game/Dev/Camera/Camera2_BP` _viewtarget
            (:`then`
              (goto _label_3))
            (:`CastFailed`
              (cast `/Game/Dev/Camera/Camera3_BP` _viewtarget
                (:`then`
                  (goto _label))
                (:`CastFailed`
                  (goto _label_2))))))))))

(fn `UserConstructionScript`
  (bind _outactors (`GameplayStatics.GetAllActorsOfClass` "/Game/Dev/Camera/Camera2_BP.Camera2_BP_C"))
  (for _array_element _outactors
    (set `self.Camera2` _array_element)
    (bind _outactors_2 (`GameplayStatics.GetAllActorsOfClass` "/Game/Dev/Camera/Camera3_BP.Camera3_BP_C"))
    (for _array_element_2 _outactors_2
      (set `self.Camera3` _array_element_2)
      (bind _outactors_3 (`GameplayStatics.GetAllActorsOfClass` "/Game/Dev/Camera/Camera4_BP.Camera4_BP_C"))
      (for _array_element_3 _outactors_3
        (set `self.Camera4` _array_element_3)
        (bind _outactors_4 (`GameplayStatics.GetAllActorsOfClass` "/Game/Dev/Camera/Camera1_BP.Camera1_BP_C"))
        (for _array_element_4 _outactors_4
          (set `self.Camera1` _array_element_4))))))