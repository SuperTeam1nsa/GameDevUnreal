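; BP_exempleLectureInventaire is an example actor showing how to read the player's inventory to check for a required item.
; On BeginPlay it waits three seconds through a gameplay task delay, then finds the first BP_Inventaire and looks up "BP_Floor" by name ID.
; If the item exists, it unhides that object and removes it from the inventory.
; An unconnected snippet sketches iterating over the full item array.
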(event `self.ReceiveBeginPlay`
  ;[1 1 1] Ici pour s'assurer dans l'exemple que le tableau ne sera pas vide
  (bind _returnvalue (`AddComponent|NODE_AddGameplayTasksComponent-0`))
  (`GameplayTask_WaitDelay.TaskWaitDelay` _returnvalue 3.0
    (:`OnFinish`
      (`KismetSystemLibrary.PrintString` "Test Lecture maintenant: réapparition du floor")
      (bind _outactors (`GameplayStatics.GetAllActorsOfClass` "/Game/BP_Inventaire.BP_Inventaire_C"))
      (bind _output (`|GetArrayItem` _outactors))
      ;[1 1 1] On cherche à savoir si le joueur a récupéré un item stratégique qu'il lui faut pour faire l'action(un téléphone pour appeler etc) et on récupère l'item(suppression de l'inventaire  selon )
      (bind (_objet _exist) (`/Game/BP_Inventaire.getItemByNameIDIfExist` _output "BP_Floor")) ; Attention l'ID peut varier du nom #check rigth
      (if _exist
        (`self.SetActorHiddenInGame` _objet false)
        (`/Game/BP_Inventaire.removeFromInventory` _output _objet)))))

(fn `UserConstructionScript`)