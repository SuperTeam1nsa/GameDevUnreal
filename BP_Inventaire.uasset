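; Inventory Blueprint that stores collected objects in a map (ArrayInventaire) keyed by each object's internal name.
; PutInInventory hides the object in game and adds it to the map.
; Getters return all stored objects or look one up by name with an existence flag.
; RemoveFromInventory does nothing because its map removal is disconnected, and the event graph holds only disabled default events.
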(fn `getArrayOfItem`
  (returns (`Array Actor` :type "Array of Actor Object Reference"))
  (bind _values (`BlueprintMapLibrary.Map_Values` (`self.ArrayInventaire`)))
  (return _values))

(fn `getItemByNameIDIfExist`
  (params (Nom :type String))
  (returns (Objet :type "Actor Object Reference") (Exist :type Boolean))
  (bind (_value _returnvalue) (`BlueprintMapLibrary.Map_Find` (`self.ArrayInventaire`) Nom))
  (return _value _returnvalue))

(fn `putInInventory`
  (params (objet :type "Actor Object Reference"))
  (`self.SetActorHiddenInGame` objet true) ; Masquage de l'objet dans le jeu
  ;[1 1 1] Ajout de l'objet à l'inventaire(map avec des strings en Keys)
  (`BlueprintMapLibrary.Map_Add` (`self.ArrayInventaire`) (`KismetSystemLibrary.GetObjectName` objet) objet))

(fn `removeFromInventory`
  (params (Objet :type "Actor Object Reference")))

(fn `UserConstructionScript`)