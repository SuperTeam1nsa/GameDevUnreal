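; Camera switcher that cycles the player's view through four fixed camera Blueprints, Camera1_BP to Camera4_BP.
; Releasing the SwitchCam input passes its key to FonctionSwitchCam, where Right steps forward and Left steps backward, wrapping around.
; The function identifies the current camera by casting player 0's view target, then finds the neighbor by class lookup and sets it with SetViewTargetWithBlend.
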(event `InputAction|SwitchCam`
  (params (Key :type "Key Structure"))
  (:`Released`
    (`self.fonction_SwitchCam` Key)))

(fn `fonction_SwitchCam`
  (params (Keys :type "Key Structure"))
  (bind _returnvalue (`GameplayStatics.GetPlayerController` 0))
  (bind _returnvalue_2 (`Controller.GetViewTarget` _returnvalue))
  (if (== Keys "Left")
    (cast `/Game/Camera1_BP` _returnvalue_2
      (:`then`
        (bind _outactors (`GameplayStatics.GetAllActorsOfClass` "/Game/Camera4_BP.Camera4_BP_C" :!label _label))
        (`PlayerController.SetViewTargetWithBlend` _returnvalue (`|GetArrayItem` _outactors) 0.0 "VTBlend_Linear" 0.0 false))
      (:`CastFailed`
        (cast `/Game/Camera2_BP` _returnvalue_2
          (:`then`
            (bind _outactors_2 (`GameplayStatics.GetAllActorsOfClass` "/Game/Camera1_BP.Camera1_BP_C" :!label _label_2))
            (`PlayerController.SetViewTargetWithBlend` _returnvalue (`|GetArrayItem` _outactors_2) 0.0 "VTBlend_Linear" 0.0 false))
          (:`CastFailed`
            (cast `/Game/Camera4_BP` _returnvalue_2
              (:`then`
                (bind _outactors_3 (`GameplayStatics.GetAllActorsOfClass` "/Game/Camera3_BP.Camera3_BP_C" :!label _label_3))
                (`PlayerController.SetViewTargetWithBlend` _returnvalue (`|GetArrayItem` _outactors_3) 0.0 "VTBlend_Linear" 0.0 false))
              (:`CastFailed`
                (bind _outactors_4 (`GameplayStatics.GetAllActorsOfClass` "/Game/Camera2_BP.Camera2_BP_C" :!label _label_4))
                (for _array_element _outactors_4
                  (`PlayerController.SetViewTargetWithBlend` _returnvalue _array_element 0.0 "VTBlend_Linear" 0.0 false))))))))
    (elif (== Keys "Right")
      (cast `/Game/Camera1_BP` _returnvalue_2
        (:`then`
          (goto _label_4))
        (:`CastFailed`
          (cast `/Game/Camera2_BP` _returnvalue_2
            (:`then`
              (goto _label_3))
            (:`CastFailed`
              (cast `/Game/Camera3_BP` _returnvalue_2
                (:`then`
                  (goto _label))
                (:`CastFailed`
                  (goto _label_2))))))))))

(fn `UserConstructionScript`)